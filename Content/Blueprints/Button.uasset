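; Numbered puzzle button that helps unlock a linked Gate when buttons are pressed in the correct order.
; PressButton swaps the Cube to a pressed material for one second, then compares its ButtonNum to the Gate's ButtonCount.
; A match advances the count and unlocks the Gate when it reaches five, while a wrong press resets the sequence to zero.
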(event `/Game/Blueprints/IPressButton.PressButton`
  (bind _gate (`self.Gate`))
  (bind _cube (`self.Cube`))
  (bind _buttoncount (`/Game/Blueprints/BigGate.ButtonCount` _gate))
  (`PrimitiveComponent.SetMaterial` _cube 0 "/Game/Materials/MaterialButtonPressed.MaterialButtonPressed")
  (`KismetSystemLibrary.Delay` 1.0)
  (`PrimitiveComponent.SetMaterial` _cube 0 "/Game/Materials/MaterialButton.MaterialButton")
  (if (== (`self.ButtonNum`) _buttoncount)
    (bind _result (`/Engine/EditorBlueprintResources/StandardMacros.IncrementInt` _buttoncount)
      (:`  `
        (bind _output_get (set `/Game/Blueprints/BigGate.ButtonCount` _result _gate))
        (if (== _output_get 5)
          (`KismetSystemLibrary.PrintString` "Unlocked Door")
          (set `/Game/Blueprints/BigGate.Locked` false _gate))))
    (else
      (set `/Game/Blueprints/BigGate.ButtonCount` 0 _gate))))

(fn `UserConstructionScript`)